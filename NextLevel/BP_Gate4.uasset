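; BP_Gate4 is an interactable gate actor that sends the player back to the Lobby level.
; A Trigger overlap with the third-person character enables the E key, which shows a fade widget, plays a sleep sound and opens Lobby after a long delay.
; A separate Sphere overlap shows a prompt widget, which starts hidden on BeginPlay and hides again when the overlap ends.
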(event OnComponentBeginOverlap(Trigger)
  (params (OverlappedComponent :type Primitive%20Component%20Object%20Reference) (OtherActor :type Actor%20Object%20Reference) (OtherComp :type Primitive%20Component%20Object%20Reference) (OtherBodyIndex :type Integer) (bFromSweep :type Boolean) (SweepResult :type Hit%20Result%20Structure%20%28by%20ref%29))
  ;[0.15 0.15 0.15 0.5] NextLevel
  (Utilities|Casting|CastToBP_ThirdPersonCharacter OtherActor)
  (bind _output_get (Variables|Default|SetbCanMove true)))

(event OnComponentEndOverlap(Trigger)
  (params (OverlappedComponent :type Primitive%20Component%20Object%20Reference) (OtherActor :type Actor%20Object%20Reference) (OtherComp :type Primitive%20Component%20Object%20Reference) (OtherBodyIndex :type Integer))
  ;[0.15 0.15 0.15 0.5] NextLevel
  (Utilities|Casting|CastToBP_ThirdPersonCharacter OtherActor)
  (Variables|Default|SetbCanMove false))

(event OnComponentBeginOverlap(Sphere)
  (params (OverlappedComponent :type Primitive%20Component%20Object%20Reference) (OtherActor :type Actor%20Object%20Reference) (OtherComp :type Primitive%20Component%20Object%20Reference) (OtherBodyIndex :type Integer) (bFromSweep :type Boolean) (SweepResult :type Hit%20Result%20Structure%20%28by%20ref%29))
  ;[0.15 0.15 0.15 0.5] E
  (Rendering|SetVisibility (Variables|Default|GetWidget) true false))

(event OnComponentEndOverlap(Sphere)
  (params (OverlappedComponent :type Primitive%20Component%20Object%20Reference) (OtherActor :type Actor%20Object%20Reference) (OtherComp :type Primitive%20Component%20Object%20Reference) (OtherBodyIndex :type Integer))
  ;[0.15 0.15 0.15 0.5] E
  (Rendering|SetVisibility (Variables|Default|GetWidget) false false))

(event EventBeginPlay
  ;[0.15 0.15 0.15 0.5] E
  (Rendering|SetVisibility (Variables|Default|GetWidget) false false))

(event Input|KeyboardEvents|E
  (params (Key :type Key%20Structure :default "None"))
  ;[0.15 0.15 0.15 0.5] NextLevel
  (:Pressed
    (if (stale OnComponentBeginOverlap(Trigger) _output_get)
      (bind _returnvalue (UserInterface|CreateWidget "/Game/NextLevel/WB_fade.WB_fade_C"))
      (UserInterface|Viewport|AddtoViewport _returnvalue 0)
      (Audio|PlaySound2D "/Game/NextLevel/SleepSound.SleepSound" 1.0 1.0 0.0 0 0)
      (Utilities|FlowControl|Delay 13.0)
      (Game|OpenLevel(byObjectReference) "/Game/Lobby.Lobby"))))

(fn ConstructionScript)