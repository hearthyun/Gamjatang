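; BP_OpenDoor is an interactable door Blueprint that swings open and closed on a Pivot component.
; Interact toggles DoorsClosed and plays or reverses the OpenCloseDoors timeline, whose Alpha sets the pivot's relative yaw.
; AnimationDone blocks input until the timeline finishes, while Issoundplay and a Delay throttle the 2D door sound fired from timeline updates.
; The IntDot event and construction script are empty.
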(event EventInteract
  (bind _pivot (Variables|Default|GetPivot))
  (bind _relativerotation (Variables|/Script/Engine.SceneComponent|GetRelativeRotation _pivot))
  (if true
    (if (Variables|Default|GetbAnimationDone?)
      (if (Variables|Default|GetbDoorsClosed?)
        (Variables|Default|SetbAnimationDone? false)
        (Variables|Default|SetbDoorsClosed? false)
        (bind _alpha (Timeline|OpenCloseDoors Play)
          (:Update
            (Transformation|SetRelativeRotation _pivot (Math|Rotator|MakeRotator (.roll _relativerotation) (.pitch _relativerotation) _alpha) false false)
            (if (Variables|Default|Getissoundplay?)
              (Audio|PlaySound2D "/Game/lockdoor/door__cut_1sec_.door__cut_1sec_" 1.0 1.0 0.0 0 0)
              (Variables|Default|Setissoundplay? false)
              (Utilities|FlowControl|Delay 1.0)
              (Variables|Default|Setissoundplay? true)))
          (:Finished
            (Variables|Default|SetbAnimationDone? true)))
        (else
          (Variables|Default|SetbAnimationDone? false)
          (Variables|Default|SetbDoorsClosed? true)
          (Timeline|OpenCloseDoors Reverse))))))

(event EventIntDot)

(fn ConstructionScript)