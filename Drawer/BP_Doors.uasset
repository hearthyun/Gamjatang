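; Interactable sliding drawer or door that toggles between open and closed on each Interact event.
; An OpenCloseDoors timeline plays forward or in reverse, writing its alpha straight to the Cube's relative Y position.
; AnimationDone blocks new interactions until the timeline finishes.
; During movement a 2D drawer sound plays, throttled by a flag and a one-second delay; IntDot is an empty event.
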(event EventBeginPlay)

(event Collision|EventActorBeginOverlap
  (params (OtherActor :type Actor%20Object%20Reference)))

(event EventInteract
  (bind _cube (Variables|Default|GetCube))
  (bind _relativelocation (Variables|/Script/Engine.SceneComponent|GetRelativeLocation _cube))
  (if (Variables|Default|GetbAnimationDone?)
    (if (Variables|Default|GetbDoorsClosed?)
      (Variables|Default|SetbAnimationDone? false)
      (Variables|Default|SetbDoorsClosed? false)
      (bind _alpha (Timeline|OpenCloseDoors Play)
        (:Update
          (Transformation|SetRelativeLocation (Variables|Default|GetCube) (Math|Vector|MakeVector (.x _relativelocation) _alpha (.z _relativelocation)) false false)
          (if (Variables|Default|Getissoundplay?)
            (Audio|PlaySound2D "/Game/Drawer/drawer.drawer" 1.0 1.0 0.0 0 0)
            (Variables|Default|Setissoundplay? false)
            (Utilities|FlowControl|Delay 1.0)
            (Variables|Default|Setissoundplay? true)))
        (:Finished
          (Variables|Default|SetbAnimationDone? true)))
      (else
        (Variables|Default|SetbAnimationDone? false)
        (Variables|Default|SetbDoorsClosed? true)
        (Timeline|OpenCloseDoors Reverse)))))

(event EventIntDot)

(fn ConstructionScript)