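; BP_BatteryPickUp is an interactable battery pickup that recharges the player's flashlight.
; On BeginPlay it caches the player as BP_ThirdPersonCharacter.
; Interact checks that the character has a flashlight and is below max battery, then adds a fixed charge without clamping, destroys the actor and plays a pickup sound.
; When either check fails, it only prints a message; IntDot is left empty.
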(event EventBeginPlay
  (bind _asbp_third_person_character (Utilities|Casting|CastToBP_ThirdPersonCharacter (Game|GetPlayerCharacter 0)))
  (Variables|Default|SetChar%20Ref _asbp_third_person_character))

(event EventInteract
  (bind _char_ref (Variables|Default|GetChar%20Ref))
  ;[0.15 0.15 0.15 0.5] batteryPickUp
  (if (Variables|/Game/ThirdPerson/Blueprints/BP_ThirdPersonCharacter.BP_ThirdPersonCharacter_C|GetHasFlashLight _char_ref)
    (if (>= (Variables|/Game/ThirdPerson/Blueprints/BP_ThirdPersonCharacter.BP_ThirdPersonCharacter_C|GetCurrentBattery _char_ref) (Variables|/Game/ThirdPerson/Blueprints/BP_ThirdPersonCharacter.BP_ThirdPersonCharacter_C|GetMaxBattery _char_ref))
      (Development|PrintString "You have max Battery. Can't  PickUp more!!" true true "(R=1.000000,G=0.000000,B=0.022203,A=1.000000)")
      (else
        (Variables|/Game/ThirdPerson/Blueprints/BP_ThirdPersonCharacter.BP_ThirdPersonCharacter_C|SetCurrentBattery (Variables|Default|GetChar%20Ref) (+ (Variables|/Game/ThirdPerson/Blueprints/BP_ThirdPersonCharacter.BP_ThirdPersonCharacter_C|GetCurrentBattery _char_ref) 1e+01))
        (Actor|DestroyActor)
        (Audio|PlaySound2D "/Game/Flash/battery_pick_up.battery_pick_up" 1.0 1.0 0.0 0 0)))
    (else
      (Development|PrintString "First you need FlashLight"))))

(event EventIntDot)

(fn ConstructionScript)