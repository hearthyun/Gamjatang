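; Anim notify that plays positional monster footstep sounds based on the surface underfoot.
; When triggered, it line traces downward from the owning actor on the Visibility channel and reads the hit's surface type.
; Water plays a water step sound and any other surface plays the default monster footstep, both at the mesh location with shared attenuation.
; No sound plays if the trace misses.
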(fn ReceivedNotify
  (params (MeshComp :type Skeletal%20Mesh%20Component%20Object%20Reference) (Animation :type Anim%20Sequence%20Base%20Object%20Reference) (EventReference :type Anim%20Notify%20Event%20Reference%20Structure%20%28by%20ref%29))
  (bind _returnvalue (Components|GetOwner MeshComp))
  (bind _returnvalue_2 (Transformation|GetWorldLocation MeshComp))
  (bind _returnvalue_3 (Transformation|GetActorLocation _returnvalue))
  ;[0.15 0.15 0.15 0.5] 3D Sound and water Sound
  (bind (_outhit _returnvalue_4) (Collision|LineTraceByChannel _returnvalue_3 (+ _returnvalue_3 (* (Transformation|GetActorUpVector _returnvalue) -2e+02)) "TraceTypeQuery1" false 0 "None"))
  (if _returnvalue_4
    (switch Utilities|FlowControl|Switch|SwitchonEPhysicalSurface (Collision|GetSurfaceType _outhit)
      (:SurfaceType_Default
        (Audio|PlaySoundatLocation "/Game/AI/BS_MonsterFoot.BS_MonsterFoot" _returnvalue_2 "0, 0, 0" 1.0 1.0 0.0 "/Game/ThirdPerson/Blueprints/FootstepAt.FootstepAt" 0 0 0))
      (:SurfaceType1
        (Audio|PlaySoundatLocation "/Game/ThirdPerson/Blueprints/MS_WaterStep.MS_WaterStep" _returnvalue_2 "0, 0, 0" 1.0 1.0 0.0 "/Game/ThirdPerson/Blueprints/FootstepAt.FootstepAt" 0 0 0))))
  (return false))