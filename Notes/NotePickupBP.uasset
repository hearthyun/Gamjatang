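; NotePickupBP is a readable note actor that toggles between lying in the world and being read on screen when interacted with.
; A Box overlap tracks whether the player is near, which gates Interact.
; Picking up plays sounds, adds a NotePickuPWidgetBPI widget to the viewport and hides the Note1 component.
; Putting down, by interacting again or leaving the box, removes the widget and restores the note with a sound.
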(event OnComponentBeginOverlap(Box)
  (params (OverlappedComponent :type Primitive%20Component%20Object%20Reference) (OtherActor :type Actor%20Object%20Reference) (OtherComp :type Primitive%20Component%20Object%20Reference) (OtherBodyIndex :type Integer) (bFromSweep :type Boolean) (SweepResult :type Hit%20Result%20Structure%20%28by%20ref%29))
  (Variables|Default|SetIsPlayerNear true))

(event OnComponentEndOverlap(Box)
  (params (OverlappedComponent :type Primitive%20Component%20Object%20Reference) (OtherActor :type Actor%20Object%20Reference) (OtherComp :type Primitive%20Component%20Object%20Reference) (OtherBodyIndex :type Integer))
  (Variables|Default|SetIsPlayerNear false)
  (if (Variables|Default|GetIsReading?)
    (CallFunction|PutDownNote)))

(event Custom|PutDownNote
  (Audio|PlaySoundatLocation 0 (Transformation|GetWorldLocation (Variables|Default|Getnote1)) "0, 0, 0" 1.0 1.0 0.0 0 0 0 0)
  (Widget|RemovefromParent (stale Custom|PickupNote _returnvalue))
  (Rendering|SetVisibility (Variables|Default|Getnote1) true false)
  (Variables|Default|SetIsReading? false))

(event Custom|Toggle%20Pickup
  (if (Variables|Default|GetIsReading?)
    (CallFunction|PutDownNote)
    (else
      (CallFunction|PickupNote)
      (Audio|PlaySound2D "/Game/Notes/note.note" 1.0 1.0 0.0 0 0))))

(event Custom|PickupNote
  (Audio|PlaySoundatLocation 0 (Transformation|GetWorldLocation (Variables|Default|Getnote1)) "0, 0, 0" 1.0 1.0 0.0 0 0 0 0)
  (bind _returnvalue (UserInterface|CreateWidget "/Game/Notes/NotePickuPWidgetBPI.NotePickuPWidgetBPI_C"))
  (UserInterface|Viewport|AddtoViewport _returnvalue 0)
  (Rendering|SetVisibility (Variables|Default|Getnote1) false false)
  (Variables|Default|SetIsReading? true))

(event EventBeginPlay)

(event Collision|EventActorBeginOverlap
  (params (OtherActor :type Actor%20Object%20Reference)))

(event EventTick
  (params (DeltaSeconds :type Float%20%28single-precision%29)))

(event EventIntDot)

(event EventInteract
  (if (Variables|Default|GetIsPlayerNear)
    (CallFunction|TogglePickup)))

(fn ConstructionScript)